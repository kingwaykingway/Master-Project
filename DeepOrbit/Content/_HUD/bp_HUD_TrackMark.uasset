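; HUD widget component that displays a w_Mark marker for a tracked actor and destroys itself when that actor is destroyed.
; A Track, Aim or Trajectory preset picks the visible mark elements at BeginPlay.
; For grappling hook HitPoints, Tick maps hook state to color and labels such as distance, lock or out of range, using DoOnce gates.
; Eye mode index and brightness feed the widget material, reapplied whenever its instance becomes valid.
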(event `self.ReceiveBeginPlay`
  (bind _asw_mark (cast `/Game/_HUD/w_Mark` (`self.GetWidget`) :!pure true))
  (bind _output_get (set `self.Widget ` (cast `/Game/_HUD/w_Mark` (`self.GetWidget`) :!pure true)))
  (bind _output_get_2 (set `/Game/_HUD/w_Mark.Tracked Actor` (`self.Tracked Actor`) _output_get))
  (add `Actor.OnDestroyed` _output_get_2 (delegate `OnDestroyed (Tracked actor)`))
  (`|ExecutionSequence`
    (:`then_0`
      (switch `/Game/_HUD/MarkPatternPreset` (`self.Preset`)
        (:`NewEnumerator0`
          (`/Game/_HUD/w_Mark.Set Component Visibilities` _asw_mark true false false false true false))
        (:`NewEnumerator1`
          (`/Game/_HUD/w_Mark.Set Component Visibilities` _asw_mark false true true true false true))
        (:`NewEnumerator2`
          (`/Game/_HUD/w_Mark.Set Component Visibilities` _asw_mark false false false true false false))))
    (:`then_1`
      (`/Game/_HUD/w_Mark.Set Color` _asw_mark (`/Game/_HUD/w_Mark.Base` _asw_mark) (`self.Default Color Override`)))
    (:`then_2`
      (bind _ashit_point (cast `/Game/_Weapons/HitPoint` (`self.Tracked Actor`))))))

(event `OnDestroyed (Tracked actor)`
  (params (DestroyedActor :type "Actor Object Reference"))
  (`self.K2_DestroyComponent` self)
  (`KismetSystemLibrary.CollectGarbage`))

(event `self.ReceiveTick`
  (params (DeltaSeconds :type "Float (single-precision)"))
  (bind _returnvalue (`self.GetMaterialInstance`))
  (`|ExecutionSequence`
    (:`then_0`
      ;[0.5 1 1] Set the eye mode index when widget material is ready.
      (`/Engine/EditorBlueprintResources/StandardMacros.IsValid` _returnvalue
        (:`Is Valid`
          (`/Engine/EditorBlueprintResources/StandardMacros.DoOnce` false :!label _label
            (:`Completed`
              (`MaterialInstanceDynamic.SetScalarParameterValue` _returnvalue "EyeModeIndex" (`self.Eye Mode Index`))
              (`MaterialInstanceDynamic.SetScalarParameterValue` _returnvalue "Brightness" (`self.Brightness`)))))
        (:`Is Not Valid`
          (goto _label :!via `Reset`))))
    (:`then_1`
      (bind _ashit_point (cast `/Game/_Weapons/HitPoint` (`self.Tracked Actor`)))
      ;[0.5 1 1] Update as grappling hook hit point mark
      (bind _asgrappling_hook (cast `/Game/_Weapons/WristEquipments/GrapplingHook` (`Actor.GetOwner` _ashit_point)))
      (switch `/Game/_Weapons/WristEquipments/GrapplingHookState` (`/Game/_Weapons/WristEquipments/GrapplingHook.State` _asgrappling_hook)
        (:`NewEnumerator0`
          (goto _label_4 :!via `Reset`))
        (:`NewEnumerator1`
          (if (`/Game/_Weapons/_Equipment.Is Homing` _asgrappling_hook)
            (`self.Update Widget State` (struct :`G` 1.0 :`A` 1.0) "Locked" true)
            (goto _label_2 :!via `Reset`)
            (else
              (bind (_hit_result_bblockinghit _hit_result_binitialoverlap _hit_result_time _hit_result_distance) (`GameplayStatics.BreakHitResult` (`/Game/_Weapons/HitPoint.Hit Result` _ashit_point)))
              (`self.Update Widget State` (struct :`G` 1.0 :`A` 1.0) "" false (`/Game/_Libraries/myStaticFunctions.Format Float to Text` (/ _hit_result_distance 100.0) 1 "" "m") true)
              (goto _label_2 :!via `Reset`))))
        (:`NewEnumerator2`
          (`/Engine/EditorBlueprintResources/StandardMacros.DoOnce` false :!label _label_2
            (:`Completed`
              (`self.Update Widget State` (struct :`R` 1.0 :`G` 1.0 :`A` 1.0) "" false "Out of Range" true))))
        (:`NewEnumerator3`
          (`/Engine/EditorBlueprintResources/StandardMacros.DoOnce` false :!label _label_3
            (:`Completed`
              (`self.Update Widget State` (struct :`R` 1.0 :`A` 1.0) "" false "Launched" true)
              (goto _label_2 :!via `Reset`))))
        (:`NewEnumerator4`
          (`/Engine/EditorBlueprintResources/StandardMacros.DoOnce` false :!label _label_4
            (:`Completed`
              (`self.Update Widget State` (struct :`R` 1.0 :`A` 1.0) "" false "Pulling" true)
              (goto _label_3 :!via `Reset`))))))))

(fn `Set Brightness`
  (params (`In brightness` :type "Float (double-precision)"))
  (bind _output_get (set `self.Brightness` `In brightness`))
  (`MaterialInstanceDynamic.SetScalarParameterValue` (`self.GetMaterialInstance`) "Brightness" _output_get))

(fn `Set Eye Mode Index`
  (params (`In Eye Mode Index` :type "Float (double-precision)"))
  (bind _output_get (set `self.Eye Mode Index` `In Eye Mode Index`))
  (`MaterialInstanceDynamic.SetScalarParameterValue` (`self.GetMaterialInstance`) "EyeModeIndex" _output_get))

(fn `Update Widget State`
  (params (`new color` :type "LinearColor Structure" :default (struct :`G` 1.0 :`A` 1.0)) (`upper text` :type Text) (`upper text visibility` :type Boolean) (`lower text` :type Text) (`lower text visibility` :type Boolean))
  (bind _widget_ (`self.Widget `))
  (bind _text_top (`/Game/_HUD/w_Mark.Text_Top` _widget_))
  (bind _text_bottom (`/Game/_HUD/w_Mark.Text_Bottom` _widget_))
  (`|ExecutionSequence`
    (:`then_0`
      (`/Game/_HUD/w_Mark.Set Color` _widget_ (`/Game/_HUD/w_Mark.Base` _widget_) `new color`))
    (:`then_1`
      (if (not (`KismetTextLibrary.TextIsEmpty` `upper text`))
        (`TextBlock.SetText` _text_top `upper text`)))
    (:`then_2`
      (`Widget.SetVisibility` _text_top (select `bool` `upper text visibility` :`false` "Hidden" :`true` "Visible" :!type "ESlateVisibility Enum")))
    (:`then_3`
      (if (not (`KismetTextLibrary.TextIsEmpty` `lower text`))
        (`TextBlock.SetText` _text_bottom `lower text`)))
    (:`then_4`
      (`Widget.SetVisibility` _text_bottom (select `bool` `lower text visibility` :`false` "Hidden" :`true` "Visible" :!type "ESlateVisibility Enum")))))