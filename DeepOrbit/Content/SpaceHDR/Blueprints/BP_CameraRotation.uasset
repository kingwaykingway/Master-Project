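; Camera rig Blueprint that rotates at a set speed while cycling HDR materials on a sky sphere.
; The construction script applies the rotation speed to RotatingMovement and the camera distance to the SpringArm.
; A looping timer async-loads the next material in a wrapping list, guarded against overlapping loads.
; On load it sets the SkySphere material and recaptures the Skylight so lighting follows the new sky.
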(event `self.ReceiveBeginPlay`
  (`KismetSystemLibrary.K2_SetTimerDelegate` (delegate `changeHDRImage`) (`self.showTimeOfHDR`) true))

(event `changeHDRImage`
  (bind _hdrmaterialslist (`self.HDRMaterialsList`))
  (if (not (`self.WaitForLoadAsset`))
    (set `self.WaitForLoadAsset` true)
    (if (not (>= (- (`KismetArrayLibrary.Array_Length` _hdrmaterialslist) 1) (`self.ImageCounter`)))
      (set `self.ImageCounter` 0))
    (bind _object (`|LoadAsset` (`|GetArrayItem` _hdrmaterialslist (`self.ImageCounter`)))
      (:`Completed`
        (bind _asmaterial_instance (cast `MaterialInstance` _object))
        (`PrimitiveComponent.SetMaterial` (`StaticMeshActor.StaticMeshComponent` (`self.skySphere`)) 0 _asmaterial_instance)
        (`/Engine/EditorBlueprintResources/StandardMacros.IncrementInt` (`self.ImageCounter`)
          (:`  `
            (`SkyLightComponent.RecaptureSky` (`SkyLight.LightComponent` (`self.Skylight`)))
            (set `self.WaitForLoadAsset` false)))))))

(fn `UserConstructionScript`
  (set `RotatingMovementComponent.RotationRate` (`KismetMathLibrary.MakeRotator` 0.0 0.0 (`self.RotationSpeed`)) (`self.RotatingMovement`))
  (set `SpringArmComponent.TargetArmLength` (`self.CameradistanceToObject`) (`self.SpringArm`)))